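; GA_Stone is a Gameplay Ability that lets the player pick a ground-targeted area and spawn a stone spell there.
; On activation it waits for user-confirmed target data with a reticle, flagging the owner as selecting an area and having the controller show the area.
; A blocking hit spawns BP_Stone with a GE_Stone effect spec and area size.
; Confirm or cancel ends the ability, which clears the selecting flag.
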(event Ability|EventActivateAbility
  (bind _returnvalue (Ability|GetOwningActorfromActorInfo))
  (bind _instigator (Variables|/Script/Engine.Actor|GetInstigator _returnvalue))
  (bind _returnvalue_2 (Pawn|GetController _instigator))
  (bind _data (|WaitTargetData :ConfirmationType "UserConfirmed" :Class "/Script/MagicSystem.MagicGameplayAbilityTargetActor" :traceRange 3e+03 :ReticleClass "/Game/MagicSystem/Blueprints/BP_Stone_Reticle.BP_Stone_Reticle_C")
    (:then
      (Class|BPICombat|INTSetIsSelectingArea(Message) _returnvalue true)
      (Class|BPICombat|INTGetAreaRefTrigger(Message) _returnvalue_2)
      (Class|BPICombat|INTSetAreaVisibility(Message) _returnvalue_2 true))
    (:ValidData
      (if (.bBlockingHit (Collision|BreakHitResult (Ability|TargetData|GetHitResultfromTargetData _data)))
        (Game|SpawnActorfromClass "/Game/MagicSystem/Blueprints/BP_Stone.BP_Stone_C" (Math|Transform|MakeTransform (.Location (Collision|BreakHitResult (Ability|TargetData|GetHitResultfromTargetData _data))) "0, 0, 0" "1.000000,1.000000,1.000000") "AlwaysSpawn" "MultiplyWithRoot" 0 5e+02 (Ability|MakeOutgoingGameplayEffectSpec "/Game/MagicSystem/Blueprints/GE_Stone.GE_Stone_C") (Variables|/Script/Engine.Actor|GetInstigator (Ability|GetOwningActorfromActorInfo)))
        (Ability|EndAbility)
        (else
          (Ability|EndAbility))))
    (:Cancelled
      (Ability|EndAbility))))

(event Ability|EventOnEndAbility
  (params (bWasCancelled :type Boolean))
  (Class|BPICombat|INTSetIsSelectingArea(Message) (Ability|GetOwningActorfromActorInfo) false))