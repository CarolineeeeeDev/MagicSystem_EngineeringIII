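; BP_Stone is a magic-system actor that applies a one-shot area Gameplay Effect around itself when it spawns.
; On BeginPlay it sphere-overlaps Pawns within StoneArea, ignoring its instigator.
; For each hit with a valid Ability System Component, the instigator's component applies the stored SpecHandle effect spec to that target.
; It has no active tick, overlap or self-destroy logic.
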(event EventBeginPlay
  (bind _outactors (Collision|SphereOverlapActors (Transformation|GetActorLocation) (Variables|Preset|GetStoneArea) (Utilities|Array|MakeArray "ObjectTypeQuery3") 0 (Utilities|Array|MakeArray (Game|GetInstigator))))
  (for _array_element _outactors
    (Utilities|IsValid (Ability|GetAbilitySystemComponent _array_element)
      (:Is%20Valid
        (GameplayEffects|ApplyGameplayEffectSpecToTarget (Ability|GetAbilitySystemComponent (Game|GetInstigator)) (Variables|Preset|GetSpec%20Handle) (Ability|GetAbilitySystemComponent _array_element))))))

(event Collision|EventActorBeginOverlap
  (params (OtherActor :type Actor%20Object%20Reference)))

(event EventTick
  (params (DeltaSeconds :type Float%20%28single-precision%29)))

(fn ConstructionScript)