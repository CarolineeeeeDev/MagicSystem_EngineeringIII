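; GA_Slow is a magic Gameplay Ability that slows pawns within a spherical area at a targeted point.
; It gets instant target data from MagicGameplayAbilityTargetActor, then manually applies GE_Ball_Cost to the owning actor's instigator.
; A sphere overlap at the hit point, or trace end without a blocking hit, applies GE_SlowStart to pawns with ability systems, ignoring the owner.
; A debug sphere marks the hit location.
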(event Ability|EventActivateAbility
  (bind _data (|WaitTargetData :ConfirmationType "Instant" :Class "/Script/MagicSystem.MagicGameplayAbilityTargetActor" :ReticleClass 0)
    (:ValidData
      (GameplayEffects|ApplyGameplayEffectToSelf :self (Ability|GetAbilitySystemComponent (Variables|/Script/Engine.Actor|GetInstigator (Ability|GetOwningActorfromActorInfo))) :GameplayEffectClass "/Game/MagicSystem/Blueprints/GE_Ball_Cost.GE_Ball_Cost_C")
      (Rendering|Debug|DrawDebugSphere (.location (Ability|TargetData|GetHitResultfromTargetData _data)) 5e+02 12 "(R=0.000000,G=0.424951,B=1.000000,A=1.000000)" 5.0 3.0)
      (bind _outactors (Collision|SphereOverlapActors (select (.bblockinghit (Ability|TargetData|GetHitResultfromTargetData _data)) (.location (Ability|TargetData|GetHitResultfromTargetData _data)) (.traceend (Ability|TargetData|GetHitResultfromTargetData _data))) 5e+02 (Utilities|Array|MakeArray "ObjectTypeQuery3") 0 (Utilities|Array|MakeArray (Ability|GetOwningActorfromActorInfo))))
      (for _array_element _outactors
        (Utilities|IsValid (Ability|GetAbilitySystemComponent _array_element)
          (:Is%20Valid
            (GameplayEffects|ApplyGameplayEffectToSelf :self (Ability|GetAbilitySystemComponent _array_element) :GameplayEffectClass "/Game/MagicSystem/Blueprints/GE_SlowStart.GE_SlowStart_C"))))
      (Ability|EndAbility))
    (:Cancelled
      (Ability|EndAbility))))

(event Ability|EventOnEndAbility
  (params (bWasCancelled :type Boolean)))